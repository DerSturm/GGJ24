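; BP_Enemy_Ranged is a rifle-wielding enemy NPC that extends its parent's attack behavior.
; On BeginPlay it spawns a rifle, attaches it to the hand socket and signals that a weapon is equipped.
; Attack plays a firing montage whose notify has the BPCAttacks component fire a damaging bullet from the weapon's location toward the target.
; Montage completion or interruption ends the attack.
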(event EventBeginPlay
  (|CallParentFunction)
  (CallFunction|EquipWeapon))

(event EventEquipWeapon
  (bind _returnvalue (Game|SpawnActorfromClass "/Game/_Kitsune/_Core/Weapons/BP_Weapon_Rifle.BP_Weapon_Rifle_C" (Transformation|GetActorTransform) "Undefined" "MultiplyWithRoot" 0 0))
  (bind _output_get (Variables|Default|SetWeaponActor _returnvalue))
  (Transformation|AttachComponentToComponent _output_get (Variables|Character|GetMesh) "hand_r_rifle_socket" "SnapToTarget" "SnapToTarget" "SnapToTarget" true)
  (Variables|Default|SetIsWieldingWeapon true)
  (Default|CallOnWeaponEquipped))

(event EventAttack
  (params (AttackTarget :type Actor%20Object%20Reference))
  ;[1 1 1] Fire rifle
  (|CallParentFunction AttackTarget)
  (bind _notifyname (Animation|Montage|PlayMontage (Variables|Character|GetMesh) "/Game/_Kitsune/Characters/DummyEnemy/Animations/Montage_Fire_Rifle_Ironsights.Montage_Fire_Rifle_Ironsights")
    (:OnCompleted
      (CallFunction|AttackEnd AttackTarget :!label _label))
    (:OnInterrupted
      (goto _label))
    (:OnNotifyBegin
      (switch name _notifyname
        (:Fire
          (Default|FireBullet (Variables|Default|GetBPC_Attacks) (Transformation|GetActorLocation (Variables|Default|GetWeaponActor)) (Transformation|GetActorLocation AttackTarget) (Utilities|Struct|MakeS_DamageInfo 15.0 "NewEnumerator2" "NewEnumerator0" false true)))))))

(fn ConstructionScript
  (|CallParentFunction))