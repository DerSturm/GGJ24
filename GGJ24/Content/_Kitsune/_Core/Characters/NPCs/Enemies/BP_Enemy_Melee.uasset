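; Melee enemy character that equips a sword, slashes at targets and can randomly block incoming hits.
; Attack plays a montage whose notify runs a forward sphere trace, damaging non-team pawns through the attacks component, and disables interruption until it ends.
; TakeDamage rolls BlockChance for blockable hits before passing damage to the damage system component.
; Blocking halts movement and starts a hold timer, which a successful block replaces with a hit-reaction montage.
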(event OnBlocked(BPC_DamageSystem)
  (params (CanBeParried :type Boolean))
  ;[1 1 1] Blocking
  (Development|PrintString "Blocked" true true "(R=1.000000,G=0.202704,B=0.000000,A=1.000000)")
  (Variables|Default|SetBlockingState "NewEnumerator2")
  (Utilities|Time|ClearandInvalidateTimerbyHandle (Variables|Default|GetHoldBlockTimer))
  (Animation|Montage|PlayMontage (Variables|Character|GetMesh) "/Game/_Kitsune/Characters/Zombie/Animations/Montage_Zombie_Hit.Montage_Zombie_Hit"
    (:OnCompleted
      _)
    (:OnInterrupted
      _))
  (CallFunction|EndBlock))

(event Custom|StartBlock
  ;[1 1 1] Blocking
  (Utilities|Time|ClearandInvalidateTimerbyHandle (Variables|Default|GetHoldBlockTimer))
  (Components|Movement|StopMovementImmediately (Variables|Character|GetCharacterMovement))
  (Variables|/Game/_Kitsune/_Core/DamageSystem/BPC_DamageSystem.BPC_DamageSystem_C|SetIsBlocking (Variables|Default|GetBPC_DamageSystem) true)
  (Variables|Default|SetBlockingState "NewEnumerator1")
  (bind _returnvalue (Utilities|Time|SetTimerbyEvent (EventDispatchers|CreateEvent :!event Custom|EndBlock) 2.0))
  (Variables|Default|SetHoldBlockTimer _returnvalue))

(event Custom|EndBlock
  ;[1 1 1] Blocking
  (Variables|/Game/_Kitsune/_Core/DamageSystem/BPC_DamageSystem.BPC_DamageSystem_C|SetIsBlocking (Variables|Default|GetBPC_DamageSystem) false)
  (Variables|Default|SetBlockingState "NewEnumerator0")
  (Default|CallOnBlockEnded))

(event EventBeginPlay
  (|CallParentFunction))

(event EventAttack
  (params (AttackTarget :type Actor%20Object%20Reference))
  (bind _returnvalue (Transformation|GetActorLocation))
  ;[1 1 1] Sword slash
  (|CallParentFunction AttackTarget)
  (bind _notifyname (Animation|Montage|PlayMontage (Variables|Character|GetMesh) "/Game/_Kitsune/Characters/Zombie/Animations/Montage_Melee_Attack.Montage_Melee_Attack")
    (:then
      (Variables|/Game/_Kitsune/_Core/DamageSystem/BPC_DamageSystem.BPC_DamageSystem_C|SetIsInterruptable (Variables|Default|GetBPC_DamageSystem) false))
    (:OnCompleted
      (CallFunction|AttackEnd AttackTarget :!label _label)
      (Variables|/Game/_Kitsune/_Core/DamageSystem/BPC_DamageSystem.BPC_DamageSystem_C|SetIsInterruptable (Variables|Default|GetBPC_DamageSystem) true))
    (:OnInterrupted
      (goto _label))
    (:OnNotifyBegin
      (switch name _notifyname
        (:Slash
          (bind (_outhits _returnvalue_2) (Collision|MultiSphereTraceForObjects _returnvalue (+ _returnvalue (* (Transformation|GetActorForwardVector) 2e+02)) 2e+01 (Utilities|Array|MakeArray "ObjectTypeQuery3") false 0 "None"))
          (if _returnvalue_2
            (Default|DamageAllNonTeamMembers (Variables|Default|GetBPC_Attacks) _outhits (Utilities|Struct|MakeS_DamageInfo 25.0 "NewEnumerator1"))))))))

(event EventEquipWeapon
  (Utilities|FlowControl|Sequence
    (:then_0
      (Default|CallOnWeaponEquipped))
    (:then_1
      (bind _returnvalue (Game|SpawnActorfromClass "/Game/_Kitsune/_Core/Weapons/BP_Weapon_Sword.BP_Weapon_Sword_C" (Transformation|GetActorTransform) "Undefined" "MultiplyWithRoot" 0 0))
      (bind _output_get (Variables|Default|SetWeaponActor _returnvalue))
      (Transformation|AttachComponentToComponent _output_get (Variables|Character|GetMesh) "RightHand_Weapon_Socket" "SnapToTarget" "SnapToTarget" "SnapToTarget" true)
      (Variables|Default|SetIsWieldingWeapon true))))

(event EventUnequipWeapon
  ;[1 1 1] play montage to put away weapon (Tutorial: https://www.youtube.com/watch?v=WFV5IewGks8&list=PLNwKK6OwH7eW1n49TW6-FmiZhqRn97cRy&index=2)
  (Actor|DestroyActor (Variables|Default|GetWeaponActor))
  (Variables|Default|SetIsWieldingWeapon false)
  (Default|CallOnWeaponUnequipped))

(fn ConstructionScript
  (|CallParentFunction))

(fn TakeDamage
  (params (DamageInfo :type S%20Damage%20Info%20Structure) (DamageCauser :type Actor%20Object%20Reference))
  (if (.CanBeBlocked (Utilities|Struct|BreakS_DamageInfo DamageInfo))
    (CallFunction|TrytoBlock))
  (bind _wasdamaged (Default|TakeDamage (Variables|Default|GetBPC_DamageSystem) DamageInfo DamageCauser))
  (return _wasdamaged))

(fn TrytoBlock
  (if (<= (Math|Random|RandomFloat) (Variables|Default|GetBlockChance))
    (CallFunction|StartBlock)))