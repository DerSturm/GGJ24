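; Mage enemy character with a fireball attack, a teleport and a self-heal, signalling the end of teleport and heal through dispatchers.
; Attack fires a spell through BPCAttacks on a montage notify.
; Teleport is a disguised fast move: it hides the mesh, ignores pawn collision and flies via AIMoveTo behind Niagara effects.
; Healing spawns an AOE at a line-trace hit, heals only the mage, and removes it when the montage ends.
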(event Custom|Teleport
  (params (Location :type Vector))
  (bind _charactermovement (Variables|Character|GetCharacterMovement))
  (bind _mesh (Variables|Character|GetMesh))
  ;[1 1 1] Teleport
  (if (not (Variables|Teleport|GetIsTeleporting))
    (Variables|Teleport|SetIsTeleporting true)
    (Pawn|Components|CharacterMovement|SetMovementMode _charactermovement "MOVE_Flying" 0)
    (Variables|/Script/Engine.CharacterMovementComponent|SetMaxFlySpeed _charactermovement 5e+03)
    (Variables|/Script/Engine.CharacterMovementComponent|SetMaxAcceleration _charactermovement 1e+05)
    (Rendering|SetVisibility _mesh false true)
    (Collision|SetCollisionResponsetoChannel (Variables|Default|GetCapsuleComponent) "ECC_Pawn" "ECR_Ignore")
    (bind _returnvalue (Niagara|SpawnSystemAttached "/Game/_Kitsune/Characters/Mage/FX/NS_TeleportStart.NS_TeleportStart" _mesh "Spine1" "0, 0, 0" "0, 0, 0" "KeepRelativeOffset" false))
    (Variables|Default|SetTeleportBodyEffect _returnvalue)
    (bind _returnvalue_2 (Niagara|SpawnSystemAttached "/Game/_Kitsune/Characters/Mage/FX/NS_TeleportTrail.NS_TeleportTrail" _mesh "Spine1" "0, 0, 0" "0, 0, 0" "KeepRelativeOffset" false))
    (Variables|Default|SetTeleportTrailEffect _returnvalue_2)
    (Animation|StopAnimMontage 0)
    (AI|AIMoveTo self Location 0 15.0 false
      (:OnSuccess
        _)
      (:OnFail
        _))
    (CallFunction|TeleportEnd)
    (else
      (Utilities|FlowControl|DelayUntilNextTick)
      (Default|CallOnTeleportEnd))))

(event Custom|TeleportEnd
  (bind _charactermovement (Variables|Character|GetCharacterMovement))
  ;[1 1 1] Teleport
  (Components|Movement|StopMovementImmediately _charactermovement)
  (Pawn|Components|CharacterMovement|SetMovementMode _charactermovement "MOVE_Walking" 0)
  (Variables|/Script/Engine.CharacterMovementComponent|SetMaxAcceleration _charactermovement 1.5e+03)
  (Rendering|SetVisibility (Variables|Character|GetMesh) true true)
  (Collision|SetCollisionResponsetoChannel (Variables|Default|GetCapsuleComponent) "ECC_Pawn" "ECR_Block")
  (Default|CallOnTeleportEnd)
  (Variables|Teleport|SetIsTeleporting false)
  (Utilities|FlowControl|Delay 0.5)
  (Utilities|FlowControl|Sequence
    (:then_0
      (bind _teleportbodyeffect (Variables|Default|GetTeleportBodyEffect)
        (:then
          (Components|DestroyComponent _teleportbodyeffect))
        (:else)))
    (:then_1
      (bind _teleporttraileffect (Variables|Default|GetTeleportTrailEffect)
        (:then
          (Components|DestroyComponent _teleporttraileffect))
        (:else)))))

(event Custom|HealOverTime
  (bind _returnvalue (Transformation|GetActorLocation))
  (Animation|Montage|PlayMontage (Variables|Character|GetMesh) "/Game/_Kitsune/Characters/Mage/Animations/Montages/Montage_Mage_Heal.Montage_Mage_Heal"
    (:then
      (bind (_outhit _returnvalue_2) (Collision|LineTraceByChannel _returnvalue (* _returnvalue "0.000000,0.000000,-1000.000000") "TraceTypeQuery1" false (Utilities|Array|MakeArray self) "None"))
      (if _returnvalue_2
        (bind _returnvalue_3 (Game|SpawnActorfromClass "/Game/_Kitsune/AOE/BP_AOE_Heal.BP_AOE_Heal_C" (Math|Transform|MakeTransform (.Location (Collision|BreakHitResult _outhit)) "0, 0, 0" "1.000000,1.000000,1.000000") "Undefined" "MultiplyWithRoot" 0 1.0 1e+01 false false true 0))
        (bind _output_get (Variables|Default|SetHealAOE _returnvalue_3))
        (EventDispatchers|AssignOnAOEOverlapActor _output_get (delegate Custom|OnHealTick))
        (else
          (Animation|StopAnimMontage 0))))
    (:OnCompleted
      (CallFunction|HealOverTimeEnded :!label _label))
    (:OnInterrupted
      (goto _label))))

(event Custom|HealOverTimeEnded
  (Default|CallOnHealOverTimeEnd)
  (bind _healaoe (Variables|Default|GetHealAOE)
    (:then
      (Actor|DestroyActor _healaoe))
    (:else)))

(event Custom|OnHealTick
  (params (Actor :type Actor%20Object%20Reference))
  (if (== Actor self)
    (CallFunction|Heal 8.0)))

(event EventBeginPlay
  (|CallParentFunction) ; This node is disabled and will not be called.\nDrag off pins to build functionality.
)

(event Collision|EventActorBeginOverlap
  (params (OtherActor :type Actor%20Object%20Reference)))

(event EventTick
  (params (DeltaSeconds :type Float%20%28single-precision%29)))

(event EventAttack
  (params (AttackTarget :type Actor%20Object%20Reference))
  (|CallParentFunction AttackTarget)
  (bind _notifyname (Animation|Montage|PlayMontage (Variables|Character|GetMesh) "/Game/_Kitsune/Characters/Mage/Animations/Montages/Montage_Mage_Fireball.Montage_Mage_Fireball")
    (:OnCompleted
      (CallFunction|AttackEnd AttackTarget))
    (:OnNotifyBegin
      (switch name _notifyname
        (:Fire
          (Default|MagicSpell (Variables|Default|GetBPC_Attacks) (Math|Transform|MakeTransform (Transformation|GetSocketLocation (Variables|Character|GetMesh) "RightHandSocket") "0, 0, 0" "1.000000,1.000000,1.000000") AttackTarget (Utilities|Struct|MakeS_DamageInfo 1e+01 "NewEnumerator2")))))))

(fn ConstructionScript
  (|CallParentFunction))

(fn SetMovementSpeed
  (params (Speed :type E_MovementSpeed%20Enum :default "NewEnumerator0"))
  (return (Utilities|Select :Index Speed :NewEnumerator0 0.0 :NewEnumerator1 (Variables|Default|GetWalkingSpeed) :NewEnumerator2 (Variables|Default|GetJoggingSpeed) :NewEnumerator3 (Variables|Default|GetSprintingSpeed))))

(fn GetIdealRange
  (return (Variables|Default|GetAttackRadius) (Variables|Default|GetDefendRadius)))