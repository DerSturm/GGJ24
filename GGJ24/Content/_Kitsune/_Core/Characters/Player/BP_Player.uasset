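; First-person player character that casts magic spells, uses jump, teleport and repulsion sphere abilities, and shows the player HUD.
; Input drives the abilities component, while right mouse holds a magic stance that changes walk speed and toggles the crosshair.
; Left mouse plays a shoot montage whose notify fires a spell from the left hand toward the camera's aim.
; A damage component backs health functions and death, block and response events, with debug keys for testing enemy AI.
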(event Custom|Death
  (Development|PrintString "YOU ARE DEAD" true true "(R=0.395833,G=0.000000,B=0.036321,A=1.000000)")
  (Input|DisableInput (Game|GetPlayerController 0)))

(event Custom|Blocked
  (params (CanBeParried :type Boolean))
  (Development|PrintString "Blocked"))

(event Custom|DamageResponse
  (params (DamageResponse :type E_DamageResponse%20Enum :default "NewEnumerator0") (DamageCauser :type Actor%20Object%20Reference))
  (Development|PrintString (Utilities|String|EnumtoString DamageResponse)))

(event Custom|EnterMagicStance
  ;[1 1 1] Change Stance
  (Variables|Combat|SetStance "NewEnumerator1")
  (Variables|/Script/Engine.CharacterMovementComponent|SetMaxWalkSpeed (Variables|Character|GetCharacterMovement) (Variables|Combat|GetMagicWalkSpeed))
  (Default|ShowCrosshair (Variables|Default|GetPlayerHUDRef)))

(event Custom|EnterDefaultStance
  ;[1 1 1] Change Stance
  (Variables|Combat|SetStance "NewEnumerator0")
  (Variables|/Script/Engine.CharacterMovementComponent|SetMaxWalkSpeed (Variables|Character|GetCharacterMovement) (Variables|Default|GetDefaultWalkSpeed))
  (Default|HideCrosshair (Variables|Default|GetPlayerHUDRef)))

(event Custom|DisplayHUD
  ;[1 1 1] HUD
  (bind _playerhudref (Variables|Default|GetPlayerHUDRef)
    (:then
      (Widget|SetVisibility _playerhudref "Visible"))
    (:else
      (bind _returnvalue (UserInterface|CreateWidget "/Game/_Kitsune/HUD/W_Player_HUD.W_Player_HUD_C" 0 0 0))
      (bind _output_get (Variables|Default|SetPlayerHUDRef _returnvalue))
      (UserInterface|Viewport|AddtoViewport _output_get 0))))

(event Input|EnhancedActionEvents|EnhancedInputActionIA_Jump
  (params (ActionValue :type Boolean) (ElapsedSeconds :type Float%20%28double-precision%29) (TriggeredSeconds :type Float%20%28double-precision%29) (InputAction :type Input%20Action%20Object%20Reference :default "/Game/_Kitsune/Input/Actions/IA_Jump.IA_Jump"))
  (Default|ActivateAbility (.BP_CharacterAbilitiesComponent (Variables|Default|GetBP_CharacterAbilitiesComponent))))

(event Input|EnhancedActionEvents|EnhancedInputActionIA_Teleport
  (params (ActionValue :type Boolean) (ElapsedSeconds :type Float%20%28double-precision%29) (TriggeredSeconds :type Float%20%28double-precision%29) (InputAction :type Input%20Action%20Object%20Reference :default "/Game/_Kitsune/Input/Actions/IA_Teleport.IA_Teleport"))
  ;[1 1 1] Abilities
  (:Triggered
    (Default|ActivateAbility :self (.BP_CharacterAbilitiesComponent (Variables|Default|GetBP_CharacterAbilitiesComponent)) :Ability "NewEnumerator5"))
  (:Canceled
    (Default|DeactivateAbility (.BP_CharacterAbilitiesComponent (Variables|Default|GetBP_CharacterAbilitiesComponent)) 0 "NewEnumerator5" :!label _label))
  (:Completed
    (goto _label)))

(event Input|EnhancedActionEvents|EnhancedInputActionIA_RepulsionSphere
  (params (ActionValue :type Boolean) (ElapsedSeconds :type Float%20%28double-precision%29) (TriggeredSeconds :type Float%20%28double-precision%29) (InputAction :type Input%20Action%20Object%20Reference :default "/Game/_Kitsune/Input/Actions/IA_RepulsionSphere.IA_RepulsionSphere"))
  ;[1 1 1] Abilities
  (:Triggered
    (Default|ActivateAbility :self (.BP_CharacterAbilitiesComponent (Variables|Default|GetBP_CharacterAbilitiesComponent)) :Ability "NewEnumerator6"))
  (:Canceled
    (Default|DeactivateAbility (.BP_CharacterAbilitiesComponent (Variables|Default|GetBP_CharacterAbilitiesComponent)) 0 "NewEnumerator6" :!label _label))
  (:Completed
    (goto _label)))

(event EventBeginPlay
  (|CallParentFunction)
  (Default|AddAbility (.BP_CharacterAbilitiesComponent (Variables|Default|GetBP_CharacterAbilitiesComponent)))
  (Default|AddAbility (.BP_CharacterAbilitiesComponent (Variables|Default|GetBP_CharacterAbilitiesComponent)) 0 "NewEnumerator5")
  (Default|AddAbility (.BP_CharacterAbilitiesComponent (Variables|Default|GetBP_CharacterAbilitiesComponent)) 0 "NewEnumerator6")
  (CallFunction|DisplayHUD))

(event Input|KeyboardEvents|DebugKeyB
  (params (Key :type Key%20Structure) (ActionValue :type Input%20Action%20Value%20Structure))
  (bind _returnvalue (Transformation|GetActorLocation))
  ;[1 1 1] Debug to interact with AI Enemy
  (:Pressed
    (Class|Actor|MakeNoise 1.0 self _returnvalue 0.0 "None")
    (Effects|SpawnEmitteratLocation "/Game/StarterContent/Particles/P_Explosion.P_Explosion" _returnvalue)
    (Audio|PlaySoundatLocation "/Game/StarterContent/Audio/Explosion01.Explosion01" _returnvalue "0, 0, 0" 1.0 1.0 0.0 0 0 0 0)))

(event Input|KeyboardEvents|DebugKeyX
  (params (Key :type Key%20Structure) (ActionValue :type Input%20Action%20Value%20Structure))
  ;[1 1 1] Debug to interact with AI Enemy
  (:Pressed
    (bind _returnvalue (Actor|GetActorOfClass "/Game/_Kitsune/_Core/Characters/NPCs/Enemies/BP_Enemy_Ranged.BP_Enemy_Ranged_C"))
    (Class|AISenseDamage|ReportDamageEvent _returnvalue self 1e+01 (Transformation|GetActorLocation) "0, 0, 0" "None")
    (Effects|SpawnEmitteratLocation "/Game/StarterContent/Particles/P_Explosion.P_Explosion" (Transformation|GetActorLocation _returnvalue))
    (Default|TakeDamage _returnvalue (Utilities|Struct|MakeS_DamageInfo 1e+01 "NewEnumerator3"))))

(event Input|MouseEvents|RightMouseButton
  (params (Key :type Key%20Structure))
  ;[1 1 1] Change Stance
  (:Pressed
    (CallFunction|EnterMagicStance))
  (:Released
    (CallFunction|EnterDefaultStance)))

(event Input|MouseEvents|LeftMouseButton
  (params (Key :type Key%20Structure))
  (bind _mesh (Variables|Character|GetMesh))
  (bind _firstpersoncameracomponent (Variables|Default|GetFirstPersonCameraComponent))
  (bind _returnvalue (Transformation|GetSocketLocation _mesh "hand_lSocket"))
  ;[1 1 1] Change Stance
  (:Pressed
    (bind _notifyname (Animation|Montage|PlayMontage 0 "/Game/_Kitsune/Characters/Player/Animation/Montage_Magic_Shoot.Montage_Magic_Shoot")
      (:OnNotifyEnd
        (switch name _notifyname
          (:Fire
            (Default|MagicSpell (Variables|Default|GetBPC_Attacks) (Math|Transform|MakeTransform _returnvalue (Math|Rotator|FindLookatRotation _returnvalue (+ (Transformation|GetWorldLocation _firstpersoncameracomponent) (* (Math|Vector|GetForwardVector _firstpersoncameracomponent) 1e+03))) "1.000000,1.000000,1.000000") 0 (Utilities|Struct|MakeS_DamageInfo 1e+01 "NewEnumerator2"))))))))

(fn ConstructionScript
  (|CallParentFunction)
  (EventDispatchers|BindEventtoOnDeath (Variables|Default|GetBPC_DamageSystem) (EventDispatchers|CreateEvent :!event Custom|Death))
  (EventDispatchers|BindEventtoOnBlocked (Variables|Default|GetBPC_DamageSystem) (EventDispatchers|CreateEvent :!event Custom|Blocked))
  (EventDispatchers|BindEventtoOnDamageResponse (Variables|Default|GetBPC_DamageSystem) (EventDispatchers|CreateEvent :!event Custom|DamageResponse)))

(fn GetCurrentHealth
  (return (Variables|/Game/_Kitsune/_Core/DamageSystem/BPC_DamageSystem.BPC_DamageSystem_C|GetHealth (Variables|Default|GetBPC_DamageSystem))))

(fn GetMaxHealth
  (return (Variables|/Game/_Kitsune/_Core/DamageSystem/BPC_DamageSystem.BPC_DamageSystem_C|GetMaxHealth (Variables|Default|GetBPC_DamageSystem))))

(fn GetTeamNumber
  (return 0))

(fn Heal
  (params (Amount :type Float%20%28double-precision%29))
  (bind _newhealth (Default|Heal (Variables|Default|GetBPC_DamageSystem) Amount))
  (return _newhealth))

(fn IsAttacking
  (return false))

(fn IsDead
  (return (Variables|/Game/_Kitsune/_Core/DamageSystem/BPC_DamageSystem.BPC_DamageSystem_C|GetIsDead (Variables|Default|GetBPC_DamageSystem))))

(fn ReserveAttackToken
  (params (Amount :type Integer))
  (return false))

(fn TakeDamage
  (params (DamageInfo :type S%20Damage%20Info%20Structure) (DamageCauser :type Actor%20Object%20Reference))
  (bind _wasdamaged (Default|TakeDamage (Variables|Default|GetBPC_DamageSystem) DamageInfo DamageCauser))
  (return _wasdamaged))