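; Base ability actor that caches its owning pawn and runs a three-state lifecycle of ready, active and cooldown.
; Activation requests pass only when ready, then store the ability info and fire an activated callback.
; Deactivation fires its callback and starts a one-shot timer that signals cooldown over and restores readiness.
; Getters expose state and cooldown ratio, though CurrentCooldown is only set to max here, never counted down.
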(event Custom|UpdateCooldown
  (Default|CallOnCooldownOver)
  (Variables|Default|SetState "NewEnumerator0"))

(event EventBeginPlay
  (bind _aspawn (Utilities|Casting|CastToPawn (Components|GetOwner)))
  (Variables|Default|SetOwningPawnRef _aspawn))

(event EventUpdateAbilityInfo
  (params (AbilityInfo :type S%20Ability%20Info%20Structure))
  (Variables|Default|SetAbilityInfo AbilityInfo))

(event EventActivateAbility
  (params (AbilityInfo :type S%20Ability%20Info%20Structure))
  (Variables|Default|SetAbilityInfo AbilityInfo)
  (Variables|Default|SetState "NewEnumerator1")
  (Variables|Default|SetCurrentCooldown (Variables|Default|GetMaxCooldown))
  (Default|CallOnActivated))

(event EventDeactivateAbility
  (Variables|Default|SetState "NewEnumerator2")
  (bind _returnvalue (Utilities|Time|SetTimerbyEvent (delegate Custom|UpdateCooldown) (Variables|Default|GetMaxCooldown)))
  (Variables|Default|SetCooldownTimer _returnvalue)
  (Default|CallOnDeactivated))

(event EventTryActivateAbility
  (params (AbilityInfo :type S%20Ability%20Info%20Structure))
  (if (Utilities|Enum|Equal(Enum) (Variables|Default|GetState) "NewEnumerator0")
    (CallFunction|ActivateAbility AbilityInfo)))

(fn ConstructionScript)

(fn GetCooldown
  (return (/ (Variables|Default|GetCurrentCooldown) (Variables|Default|GetMaxCooldown))))

(fn GetStatus
  (return (Variables|Default|GetState)))