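; BP_Ability_RepulsionSphere is a charged ability, attached to its owning pawn, that releases a radial physics push.
; Activation plays a timeline that grows force and radius toward their maximums while drawing a debug sphere.
; Deactivation, manual or on timeline finish, passes a DoOnce re-armed per activation, stops the timeline and fires the push.
; The push applies a linear-falloff radial impulse to overlapping PhysicsBody static mesh actors.
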(event Custom|DoForcePush
  (bind _returnvalue (Transformation|GetActorLocation))
  (bind _outactors (Collision|SphereOverlapActors (Transformation|GetActorLocation) (Variables|Default|GetcurrentRadius) (Utilities|Array|MakeArray "ObjectTypeQuery4") 0))
  (for _array_element _outactors
    (bind _asstatic_mesh_actor (Utilities|Casting|CastToStaticMeshActor _array_element))
    (Physics|AddRadialImpulse (Variables|/Script/Engine.StaticMeshActor|GetStaticMeshComponent _asstatic_mesh_actor) _returnvalue (Variables|Default|GetcurrentRadius) (Variables|Default|GetcurrentForce) "RIF_Linear" false)
    (Rendering|Debug|DrawDebugSphere _returnvalue (Variables|Default|GetcurrentRadius) 12 "(R=1.000000,G=1.000000,B=1.000000,A=1.000000)" 2.0 2.0)))

(event EventBeginPlay
  (|CallParentFunction)
  (Transformation|AttachActorToActor (Variables|Default|GetOwningPawnRef) "None" "KeepRelative" "KeepRelative" "KeepRelative" true))

(event EventActivateAbility
  (params (AbilityInfo :type S%20Ability%20Info%20Structure))
  (Utilities|FlowControl|Sequence
    (:then_0
      (|CallParentFunction AbilityInfo)
      (bind (_direction _forceincrease _radiusincrease) (Timeline|RepulsionSphere PlayFromStart)
        (:Update
          (Variables|Default|SetcurrentForce (* _forceincrease (Variables|Default|GetMaxForce)))
          (bind _output_get (Variables|Default|SetcurrentRadius (* (Variables|Default|GetMaxRadius) _radiusincrease)))
          (Rendering|Debug|DrawDebugSphere (Transformation|GetActorLocation (.OwningPawn (Utilities|Struct|BreakS_AbilityInfo AbilityInfo))) _output_get 12 "(R=1.000000,G=1.000000,B=1.000000,A=1.000000)" 0.0 2.0))
        (:Finished
          (CallFunction|DeactivateAbility))))
    (:then_1
      (Utilities|FlowControl|DoOnce false) ; enters at Reset
    )))

(event EventDeactivateAbility
  (Utilities|FlowControl|DoOnce false
    (:Completed
      (Utilities|FlowControl|Sequence
        (:then_0
          (bind (_direction _forceincrease _radiusincrease) (Timeline|RepulsionSphere Stop)
            (:Update
              (Variables|Default|SetcurrentForce (* _forceincrease (Variables|Default|GetMaxForce)))
              (bind _output_get (Variables|Default|SetcurrentRadius (* (Variables|Default|GetMaxRadius) _radiusincrease)))
              (Rendering|Debug|DrawDebugSphere (Transformation|GetActorLocation (.OwningPawn (Utilities|Struct|BreakS_AbilityInfo (stale EventActivateAbility AbilityInfo)))) _output_get 12 "(R=1.000000,G=1.000000,B=1.000000,A=1.000000)" 0.0 2.0))
            (:Finished
              (CallFunction|DeactivateAbility))))
        (:then_1
          (|CallParentFunction)
          (CallFunction|DoForcePush))))))

(fn ConstructionScript
  (|CallParentFunction))