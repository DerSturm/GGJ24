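; Jetpack ability that thrusts the owning character upward while burning a limited fuel supply, which starts full at BeginPlay.
; On activation with fuel left, it sets the character's air control, immediately deactivates the ability, then plays a thrust timeline.
; Each timeline update launches the character vertically by the curve value times power and drains fuel, stopping when empty.
; Nothing in this graph refills fuel or restores air control.
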(event EventBeginPlay
  (|CallParentFunction)
  (Variables|Default|SetFuel (Variables|Default|GetMaxFuel)))

(event EventDeactivateAbility
  (|CallParentFunction))

(event EventActivateAbility
  (params (AbilityInfo :type S%20Ability%20Info%20Structure))
  (|CallParentFunction AbilityInfo)
  (if (> (Variables|Default|GetFuel) 0.0)
    (bind _ascharacter (Utilities|Casting|CastToCharacter (.OwningPawn (Utilities|Struct|BreakS_AbilityInfo AbilityInfo))))
    (Variables|Default|SetOwningCharacterRef _ascharacter)
    (Variables|/Script/Engine.CharacterMovementComponent|SetAirControl (Variables|/Script/Engine.Character|GetCharacterMovement _ascharacter) (Variables|Default|GetAirControl))
    (CallFunction|DeactivateAbility)
    (bind _thrust (Timeline|TL_Thrust PlayFromStart)
      (:Update
        (Character|LaunchCharacter (Variables|Default|GetOwningCharacterRef) (Math|Vector|MakeVector 0.0 0.0 (* _thrust (Variables|Default|GetPower))) false false)
        (bind _output_get (Variables|Default|SetFuel (- (Variables|Default|GetFuel) (Variables|Default|GetFuelConsumptionRate))))
        (if (<= _output_get 0.0)
          (Timeline|TL_Thrust Stop)
          (else
            (Character|StopJumping (Variables|Default|GetOwningCharacterRef))))))))

(fn ConstructionScript
  (|CallParentFunction))