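; Ability component that tracks activation status and cooldown for an ability, exposing both through getters.
; Activation succeeds only from the default status, switching it and firing the activated dispatcher; otherwise it prints a cooldown message.
; Deactivation waits for the cooldown time, then restores the status and fires the deactivated dispatcher.
; The Tick status check and an ability-info struct builder are unfinished stubs.
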(event EventBeginPlay)

(event EventTick
  (params (DeltaSeconds :type Float%20%28single-precision%29))
  (if (Utilities|Enum|Equal(Enum) (Variables|Default|GetAbilityStatus) "NewEnumerator1")
    _))

(event EventDeactivateAbility
  (Utilities|FlowControl|Delay (Variables|Default|GetCooldownTime))
  (Variables|Default|SetAbilityStatus "NewEnumerator0")
  (Default|CallOnAbilityDeactivated))

(event EventActivateAbility
  (params (AbilityInfo :type S%20Ability%20Info%20Structure))
  (if (Utilities|Enum|Equal(Enum) (Variables|Default|GetAbilityStatus) "NewEnumerator0")
    (Variables|Default|SetAbilityStatus "NewEnumerator1")
    (Default|CallOnAbilityActivated)
    (else
      (Development|PrintString "This ability is still on cooldown"))))

(fn GetCooldown
  (return (Variables|Default|GetCooldownTime)))

(fn GetStatus
  (return (Variables|Default|GetAbilityStatus)))