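; Teleport ability that previews a grounded destination with a target marker and moves the owning pawn there on deactivation.
; Activation and Tick feed the cast location and direction into a placement check, which traces out to max distance, then vertically around that point to find ground.
; A ground hit spawns or moves the marker, a miss destroys it, and deactivation teleports only if the marker exists, destroying it.
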(event EventBeginPlay
  (|CallParentFunction))

(event EventActivateAbility
  (params (AbilityInfo :type S%20Ability%20Info%20Structure))
  (bind _output_get (Variables|Default|SetAbilityInfo AbilityInfo))
  (|CallParentFunction _output_get)
  (bind (_placeable _groundedposition _target) (CallFunction|TrytoPlaceTarget (.CastLocation (Utilities|Struct|BreakS_AbilityInfo _output_get)) (.CastDirection (Utilities|Struct|BreakS_AbilityInfo _output_get))))
  (Variables|Default|SetTargetLocation _groundedposition)
  (if _placeable
    (Variables|Default|SetTargetPointRef _target)))

(event EventDeactivateAbility
  (bind _targetpointref (Variables|Default|GetTargetPointRef))
  (Utilities|IsValid _targetpointref
    (:Is%20Valid
      (Variables|Default|SetTargetLocation (Transformation|GetActorLocation _targetpointref))
      (Actor|DestroyActor _targetpointref)
      (Transformation|SetActorLocation (Variables|Default|GetOwningPawnRef) (Variables|Default|GetTargetLocation) false true))))

(event EventTick
  (params (DeltaSeconds :type Float%20%28single-precision%29))
  (bind _abilityinfo (Variables|Default|GetAbilityInfo))
  (bind (_type _owningpawn _castlocation _castdirection) (Utilities|Struct|BreakS_AbilityInfo _abilityinfo))
  (bind _groundedposition (CallFunction|TrytoPlaceTarget _castlocation _castdirection))
  (Variables|Default|SetTargetLocation _groundedposition))

(fn ConstructionScript
  (|CallParentFunction))

(fn TrytoPlaceTarget
  (params (Location :type Vector) (Direction :type Vector))
  (bind _output_get (LocalVariables|SettargetLocation (+ Location (* Direction (Variables|Default|GetMaxDistance)))))
  (bind (_outhit _returnvalue) (Collision|LineTraceByChannel Location _output_get "TraceTypeQuery1" false (Utilities|Array|MakeArray (Components|GetOwner)) "None"))
  (if _returnvalue
    (LocalVariables|SettargetLocation (.Location (Collision|BreakHitResult _outhit))))
  ;[1 1 1] Trace downwards from first hit or at max distance
  (bind (_outhit_2 _returnvalue_2) (Collision|LineTraceByChannel (+ (LocalVariables|GettargetLocation) (Math|Vector|MakeVector 0.0 0.0 (LocalVariables|GetmaxHeight))) (+ (LocalVariables|GettargetLocation) (Math|Vector|MakeVector 0.0 0.0 (* (LocalVariables|GetmaxHeight) -1.0))) "TraceTypeQuery1" false 0 "None"))
  (if _returnvalue_2
    (Variables|Default|SetTargetLocation (.Location (Collision|BreakHitResult _outhit_2)))
    (Utilities|IsValid (Variables|Default|GetTargetPointRef)
      (:Is%20Valid
        (Transformation|SetActorLocation (Variables|Default|GetTargetPointRef) (Variables|Default|GetTargetLocation) false false))
      (:Is%20Not%20Valid
        (bind _returnvalue_3 (Game|SpawnActorfromClass "/Game/_Kitsune/Abilities/Teleport/BP_TeleportTarget.BP_TeleportTarget_C" (Math|Transform|MakeTransform (Variables|Default|GetTargetLocation)) "Undefined" "MultiplyWithRoot" 0 0))
        (bind _output_get_2 (Variables|Default|SetTargetPointRef _returnvalue_3))))
    (return _returnvalue_2 (Variables|Default|GetTargetLocation) _output_get_2)
    (else
      (Utilities|IsValid (Variables|Default|GetTargetPointRef)
        (:Is%20Valid
          (Actor|DestroyActor (Variables|Default|GetTargetPointRef))
          (return false "0, 0, 0" 0))))))