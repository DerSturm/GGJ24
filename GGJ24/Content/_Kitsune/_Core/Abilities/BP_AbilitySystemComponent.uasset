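; Custom ability system component that manages the abilities of its owning Character, warning on BeginPlay if attached to anything else.
; AddAbility spawns each ability class as an actor owned by the component's owner and stores it in CurrentAbilities.
; Remove, activate, deactivate and info-update calls find the instance by exact class and forward to it.
; RemoveAbility only drops the array entry, without destroying the spawned actor.
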(event EventBeginPlay
  (bind _ascharacter (Utilities|Casting|CastToCharacter (Components|GetOwner))
    (:then
      (Variables|Default|SetCharacterRef _ascharacter))
    (:CastFailed
      (Development|PrintString "Do not attach this component to non-characters!"))))

(event EventTick
  (params (DeltaSeconds :type Float%20%28single-precision%29)))

(fn AddAbility
  (params (Ability :type BP%20Ability%20Base%20Class%20Reference))
  (bind _returnvalue (Game|SpawnActorfromClass Ability (Math|Transform|MakeTransform "0, 0, 0" "0, 0, 0" "1.000000,1.000000,1.000000") "Undefined" "MultiplyWithRoot" (Components|GetOwner) 0))
  (Utilities|Array|AddUnique (Variables|Default|GetCurrentAbilities) _returnvalue))

(fn RemoveAbility
  (params (Ability :type BP%20Ability%20Base%20Class%20Reference))
  (bind _ability (Utilities|FindAbilitybyClass Ability)
    (:Success
      (Utilities|Array|RemoveItem (Variables|Default|GetCurrentAbilities) _ability))))

(fn ActivateAbility
  (params (Ability :type BP%20Ability%20Base%20Class%20Reference) (AbilityInfo :type S%20Ability%20Info%20Structure))
  (bind _ability (Utilities|FindAbilitybyClass Ability)
    (:Success
      (Default|TryActivateAbility _ability AbilityInfo))))

(fn DeactivateAbility
  (params (Ability :type BP%20Ability%20Base%20Class%20Reference))
  (bind _ability (Utilities|FindAbilitybyClass Ability)
    (:Success
      (Default|DeactivateAbility _ability))))

(fn UpdateAbilityInfo
  (params (Ability :type BP%20Ability%20Base%20Class%20Reference) (AbilityInfo :type S%20Ability%20Info%20Structure))
  (bind _ability (Utilities|FindAbilitybyClass Ability)
    (:Success
      (Default|UpdateAbilityInfo _ability AbilityInfo))))