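; Slam jump ability, built on a base ability, that plays a leap-smash montage on the third-person character with player input disabled.
; The montage completing or being interrupted deactivates the ability, restoring input and clearing the hit timer.
; HitActorsInRange sphere-traces forward along the character's Schlong component over SwordRange and damages BP_Enemy_Base actors.
; The looping timer and trace toggles that would drive hit detection are unconnected here.
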(event Custom|HitActorsInRange
  (bind _owningpawnref (Variables|Default|GetOwningPawnRef))
  (bind _returnvalue (Transformation|GetActorLocation _owningpawnref))
  (bind (_outhits _returnvalue_2) (Collision|MultiSphereTraceForObjects _returnvalue (+ _returnvalue (* (Math|Vector|GetForwardVector (Variables|Default|GetSchlong)) (Variables|Default|GetSwordRange))) 2e+02 (Utilities|Array|MakeArray "ObjectTypeQuery3" "ObjectTypeQuery2") false (Utilities|Array|MakeArray (Variables|Default|GetOwningPawnRef)) "None"))
  (if _returnvalue_2
    (for _array_element _outhits
      (bind _asbp_enemy_base (Utilities|Casting|CastToBP_Enemy_Base (.HitActor (Collision|BreakHitResult _array_element))))
      (Default|TakeDamage _asbp_enemy_base (Utilities|Struct|MakeS_DamageInfo 1e+02 "NewEnumerator1") self))))

(event EventBeginPlay
  (|CallParentFunction)
  (bind _asbp_third_person_character (Utilities|Casting|CastToBP_ThirdPersonCharacter (Variables|Default|GetOwningPawnRef)))
  (Variables|Default|SetSchlong (Variables|/Game/ThirdPerson/Blueprints/BP_ThirdPersonCharacter.BP_ThirdPersonCharacter_C|GetSchlong _asbp_third_person_character)))

(event EventActivateAbility
  (params (AbilityInfo :type S%20Ability%20Info%20Structure))
  (|CallParentFunction AbilityInfo)
  (Input|DisableInput (Game|GetPlayerController 0))
  (bind _asbp_third_person_character (Utilities|Casting|CastToBP_ThirdPersonCharacter (Variables|Default|GetOwningPawnRef)))
  (Animation|Montage|PlayMontage (Variables|/Script/Engine.Character|GetMesh _asbp_third_person_character) "/Game/_GGJ24/Characters/Lady_Longschlong/Animations/Locomotion/LLS_LeapSmash.LLS_LeapSmash"
    (:OnCompleted
      _)
    (:OnInterrupted
      _))
  (CallFunction|DeactivateAbility))

(event EventDeactivateAbility
  (|CallParentFunction)
  (Input|EnableInput (Game|GetPlayerController 0))
  (Utilities|Time|ClearandInvalidateTimerbyHandle (Variables|Default|GetOverTimeHitTimer)))

(fn ConstructionScript
  (|CallParentFunction))