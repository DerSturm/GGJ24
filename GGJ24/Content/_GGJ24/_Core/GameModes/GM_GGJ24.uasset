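; Game mode for GGJ24 that runs a countdown round with a score, game-over screen and pause menu.
; A looping one-second timer decrements the time remaining and updates the HUD, with events to add time or score.
; At zero it shows the end screen with the score and pauses; GameOver is set false there, so only pausing halts the countdown.
; Pause toggles the menu, game pause, cursor and input mode.
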(event Custom|UpdateTimer
  (if (not (Variables|Default|GetGameOver?))
    (bind _result (Math|Integer|DecrementInt (Variables|Default|GetTimeRemaining))
      (:%20%20
        (bind _output_get (Variables|Default|SetTimeRemaining _result))
        (if (> _output_get 0)
          (CallFunction|UpdateTimerUI)
          (else
            (CallFunction|GameOver)))))))

(event Custom|GameOver
  (bind _returnvalue (Game|GetPlayerController 0))
  (Variables|Default|SetGameOver? false)
  (bind _returnvalue_2 (UserInterface|CreateWidget "/Game/_GGJ24/_Core/UI/WBP_EndGameScreen.WBP_EndGameScreen_C" 0 (Variables|Default|GetScore)))
  (UserInterface|Viewport|AddtoViewport _returnvalue_2 0)
  (Game|SetGamePaused true)
  (Variables|/Script/Engine.PlayerController|SetbShowMouseCursor _returnvalue true)
  (Input|SetInputModeUIOnly _returnvalue 0 "DoNotLock" false))

(event Custom|AddToScore
  (params (Addition :type Integer))
  (bind _output_get (Variables|Default|SetScore (+ Addition (Variables|Default|GetScore))))
  (Default|UpdateScore (Variables|Default|GetHud) _output_get))

(event Custom|AddToTimer
  (params (Amount :type Integer))
  (Variables|Default|SetTimeRemaining (+ Amount (Variables|Default|GetTimeRemaining)))
  (CallFunction|UpdateTimerUI))

(event Custom|UpdateTimerUI
  (Default|UpdateTimer (Variables|Default|GetHud) (Variables|Default|GetTimeRemaining)))

(event Custom|Unpause
  (bind _returnvalue (Game|GetPlayerController 0))
  (Game|SetGamePaused false)
  (Variables|/Script/Engine.PlayerController|SetbShowMouseCursor _returnvalue false)
  (Input|SetInputModeGameOnly _returnvalue false)
  (Widget|RemovefromParent (Variables|Default|GetPauseMenu)))

(event Custom|Pause
  (bind _returnvalue (Game|GetPlayerController 0))
  (if (not (Game|IsGamePaused))
    (bind _returnvalue_2 (UserInterface|CreateWidget "/Game/_GGJ24/_Core/UI/WBP_PauseMenu.WBP_PauseMenu_C"))
    (bind _output_get (Variables|Default|SetPauseMenu _returnvalue_2))
    (UserInterface|Viewport|AddtoViewport _returnvalue_2 0)
    (Game|SetGamePaused true)
    (Variables|/Script/Engine.PlayerController|SetbShowMouseCursor _returnvalue true)
    (Input|SetInputModeUIOnly _returnvalue 0 "DoNotLock" false)
    (else
      (CallFunction|Unpause))))

(event EventBeginPlay
  (Utilities|Time|SetTimerbyEvent (delegate Custom|UpdateTimer) 1.0 true)
  (bind _returnvalue (UserInterface|CreateWidget "/Game/_GGJ24/_Core/UI/HUD.HUD_C"))
  (UserInterface|Viewport|AddtoViewport _returnvalue 0)
  (Variables|Default|SetHud _returnvalue)
  (CallFunction|UpdateTimerUI))

(fn ConstructionScript)