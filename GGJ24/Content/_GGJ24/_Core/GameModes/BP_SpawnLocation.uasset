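; BP_SpawnLocation is a spawn point that periodically creates melee enemies at its own location.
; On BeginPlay a looping five-second timer fires SpawnMale, which spawns BP_Enemy_Melee while MalesFromMe is below MaxAmountAtLocation.
; The counter only increments in this file, so the cap limits total spawns from the point rather than how many are alive.
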(event Custom|SpawnMale
  (if (< (Variables|Default|GetMalesFromMe) (Variables|Default|GetMaxAmountAtLocation))
    (Game|SpawnActorfromClass "/Game/_GGJ24/_Core/Characters/NPCs/Enemies/BP_Enemy_Melee.BP_Enemy_Melee_C" (Math|Conversions|ToTransform(Vector) (Transformation|GetActorLocation)) "Undefined" "MultiplyWithRoot" 0 2 0)
    (bind _result (Math|Integer|IncrementInt (Variables|Default|GetMalesFromMe))
      (:%20%20
        (Variables|Default|SetMalesFromMe _result)))))

(event EventBeginPlay
  (Utilities|Time|SetTimerbyEvent (delegate Custom|SpawnMale) 5.0 true))

(fn ConstructionScript)