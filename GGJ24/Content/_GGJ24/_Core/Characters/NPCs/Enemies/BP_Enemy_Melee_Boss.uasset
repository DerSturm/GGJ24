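; Melee boss enemy Blueprint that adds a health bar, montage-driven attacks and random blocking to its parent class.
; Attacks are uninterruptible, using a montage notify to sphere-trace forward and damage non-team pawns through the attacks component.
; Blockable incoming damage can trigger a timed, stationary block before reaching the damage system; a successful block plays a reaction, then ends blocking.
; Equipping is only a montage and flag; unequipping is unimplemented.
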(event OnBlocked(BPC_DamageSystem)
  (params (CanBeParried :type Boolean))
  ;[1 1 1] Blocking
  (Development|PrintString "Blocked" true true "(R=1.000000,G=0.202704,B=0.000000,A=1.000000)")
  (Variables|Default|SetBlockingState "NewEnumerator2")
  (Utilities|Time|ClearandInvalidateTimerbyHandle (Variables|Default|GetHoldBlockTimer))
  (Animation|Montage|PlayMontage (Variables|Character|GetMesh) 0
    (:OnCompleted
      _)
    (:OnInterrupted
      _))
  (CallFunction|EndBlock))

(event Custom|StartBlock
  ;[1 1 1] Blocking
  (Utilities|Time|ClearandInvalidateTimerbyHandle (Variables|Default|GetHoldBlockTimer))
  (Components|Movement|StopMovementImmediately (Variables|Character|GetCharacterMovement))
  (Variables|/Game/_GGJ24/_Core/DamageSystem/BPC_DamageSystem.BPC_DamageSystem_C|SetIsBlocking (Variables|Default|GetBPC_DamageSystem) true)
  (Variables|Default|SetBlockingState "NewEnumerator1")
  (bind _returnvalue (Utilities|Time|SetTimerbyEvent (EventDispatchers|CreateEvent :!event Custom|EndBlock) 2.0))
  (Variables|Default|SetHoldBlockTimer _returnvalue))

(event Custom|EndBlock
  ;[1 1 1] Blocking
  (Variables|/Game/_GGJ24/_Core/DamageSystem/BPC_DamageSystem.BPC_DamageSystem_C|SetIsBlocking (Variables|Default|GetBPC_DamageSystem) false)
  (Variables|Default|SetBlockingState "NewEnumerator0")
  (Default|CallOnBlockEnded))

(event EventBeginPlay
  (|CallParentFunction)
  (bind _returnvalue (UserInterface|CreateWidget "/Game/_GGJ24/_Core/DamageSystem/W_HealthBar.W_HealthBar_C" 0 self))
  (UserInterface|SetWidget (Variables|Default|GetHealthbar) _returnvalue))

(event EventAttack
  (params (AttackTarget :type Actor%20Object%20Reference))
  (bind _returnvalue (Transformation|GetActorLocation))
  ;[1 1 1] Sword slash
  (Development|PrintString "Attck")
  (|CallParentFunction AttackTarget)
  (bind _notifyname (Animation|Montage|PlayMontage (Variables|Character|GetMesh) "/Game/_GGJ24/Characters/Man/anims/Zombie_Headbutt_Montage.Zombie_Headbutt_Montage")
    (:then
      (Variables|/Game/_GGJ24/_Core/DamageSystem/BPC_DamageSystem.BPC_DamageSystem_C|SetIsInterruptable (Variables|Default|GetBPC_DamageSystem) false))
    (:OnCompleted
      (CallFunction|AttackEnd AttackTarget :!label _label)
      (Variables|/Game/_GGJ24/_Core/DamageSystem/BPC_DamageSystem.BPC_DamageSystem_C|SetIsInterruptable (Variables|Default|GetBPC_DamageSystem) true))
    (:OnInterrupted
      (goto _label))
    (:OnNotifyBegin
      (switch name _notifyname
        (:Slash
          (bind (_outhits _returnvalue_2) (Collision|MultiSphereTraceForObjects _returnvalue (+ _returnvalue (* (Transformation|GetActorForwardVector) 2e+02)) 2e+01 (Utilities|Array|MakeArray "ObjectTypeQuery3") false 0 "None"))
          (if _returnvalue_2
            (Default|DamageAllNonTeamMembers (Variables|Default|GetBPC_Attacks) _outhits (Utilities|Struct|MakeS_DamageInfo 25.0 "NewEnumerator1"))))))))

(event EventEquipWeapon
  (Animation|Montage|PlayMontage (Variables|Character|GetMesh) "/Game/_GGJ24/Characters/Man/anims/M_Surprised.M_Surprised"
    (:OnCompleted
      (Variables|Default|SetIsWieldingWeapon true)
      (Default|CallOnWeaponEquipped))))

(event EventUnequipWeapon)

(fn ConstructionScript
  (|CallParentFunction))

(fn TakeDamage
  (params (DamageInfo :type S%20Damage%20Info%20Structure) (DamageCauser :type Actor%20Object%20Reference))
  (if (.CanBeBlocked (Utilities|Struct|BreakS_DamageInfo DamageInfo))
    (CallFunction|TrytoBlock))
  (bind _wasdamaged (Default|TakeDamage (Variables|Default|GetBPC_DamageSystem) DamageInfo DamageCauser))
  (return _wasdamaged))

(fn TrytoBlock
  (if (<= (Math|Random|RandomFloat) (Variables|Default|GetBlockChance))
    (CallFunction|StartBlock)))