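; BP_PatrolRoute is a spline-based patrol path for enemy AI that serves the current waypoint as a world position.
; IncrementPatrolRoute steps the point index by the current direction, either wrapping around when looping or reversing at the first and last points to ping-pong.
; GetSplinePointAsWorldPosition returns the spline location at that index, and SwitchDirection flips the travel direction on demand.
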(event Custom|IncrementPatrolRoute
  (Variables|Default|SetPatrolIndex (+ (Variables|Default|GetPatrolIndex) (Variables|Default|GetDirection)))
  (if (Variables|Default|GetLooping)
    (if (== (Variables|Default|GetPatrolIndex) (Spline|GetNumberOfSplinePoints (Variables|Default|GetPatrolRoute)))
      (Variables|Default|SetPatrolIndex 0)
      (elif (== (Variables|Default|GetPatrolIndex) -1)
        (Variables|Default|SetPatrolIndex (- (Spline|GetNumberOfSplinePoints (Variables|Default|GetPatrolRoute)) 1))))
    (elif (== (Variables|Default|GetPatrolIndex) (- (Spline|GetNumberOfSplinePoints (Variables|Default|GetPatrolRoute)) 1))
      (Variables|Default|SetDirection -1)
      (elif (== (Variables|Default|GetPatrolIndex) 0)
        (Variables|Default|SetDirection 1)))))

(fn ConstructionScript)

(fn GetSplinePointasWorldPosition
  (return (Spline|GetLocationatSplinePoint (Variables|Default|GetPatrolRoute) (Variables|Default|GetPatrolIndex) "World")))

(fn SwitchDirection
  (Variables|Default|SetDirection (* (Variables|Default|GetDirection) -1)))